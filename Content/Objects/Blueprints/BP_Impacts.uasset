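; BP_Impacts is a component that plays a rock impact sound when its owning actor takes a hard hit.
; On BeginPlay it enables rigid body collision notifications on the owner's primitive root and binds to the owner's hit event.
; Hits whose impulse magnitude exceeds UpperThan play an attenuated sound at the owner's location after a short Delay, which also absorbs repeat hits while pending.
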(event Custom|HitEvent
  (params (SelfActor :type Actor%20Object%20Reference) (OtherActor :type Actor%20Object%20Reference) (NormalImpulse :type Vector) (Hit :type Hit%20Result%20Structure%20%28by%20ref%29))
  (if (> (Math|Vector|VectorLength NormalImpulse) (Variables|Default|GetUpperThan))
    (Utilities|FlowControl|Delay 0.2)
    (Audio|SpawnSoundatLocation "/Game/Objects/Sound_effects/Rock_impact/Rock_Impact.Rock_Impact" (Transformation|GetActorLocation (Components|GetOwner)) "0, 0, 0" 1.0 1.0 0.0 "/Game/Objects/Sound_effects/Rock_impact/blockAttenuation.blockAttenuation" 0)))

(event EventBeginPlay
  (bind _asprimitive_component (Utilities|Casting|CastToPrimitiveComponent (Variables|/Script/Engine.Actor|GetRootComponent (Components|GetOwner))))
  (Class|PrimitiveComponent|SetNotifyRigidBodyCollision _asprimitive_component true)
  (Collision|BindEventtoOnActorHit (Components|GetOwner) (delegate Custom|HitEvent)))