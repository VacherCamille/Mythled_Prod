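; PlayerController_BP is a player controller that opens the pause menu when the Pause input is pressed outside the menu level.
; BeginPlay adds a post-process component as PauseBlur and disables it.
; Pressing Pause pauses the game, adds the Pause widget and shows the cursor, but sets PauseBlur disabled, so no blur appears.
; An unpause chain keyed on NotPause is left unconnected and never runs.
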(event EventBeginPlay
  (bind _returnvalue (AddComponent|AddPostProcessComponent false))
  (bind _output_get (Variables|Default|SetPauseBlur _returnvalue))
  (Variables|/Script/Engine.PostProcessComponent|SetbEnabled _output_get false))

(event EventTick
  (params (DeltaSeconds :type Float%20%28single-precision%29)))

(event Input|ActionEvents|InputActionPause
  (params (Key :type Key%20Structure))
  (:Pressed
    (bind _returnvalue (Game|GetCurrentLevelName true))
    (if (not (Utilities|Enum|Equal(Enum) _returnvalue (Variables|Default|GetMenuName)))
      (Game|SetGamePaused true)
      (Variables|/Script/Engine.PostProcessComponent|SetbEnabled (Variables|Default|GetPauseBlur) false)
      (bind _returnvalue_2 (UserInterface|CreateWidget "/Game/Levels/UI/Pause.Pause_C"))
      (UserInterface|Viewport|AddtoViewport _returnvalue_2 0)
      (Variables|/Script/Engine.PlayerController|SetbShowMouseCursor (Game|GetPlayerController 0) true))))

(fn ConstructionScript)