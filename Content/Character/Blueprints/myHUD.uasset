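; HUD Blueprint that draws a simple magenta crosshair near the center of the screen.
; Each DrawHUD event draws two thin rectangles, one horizontal and one vertical, to form the cross.
; Their positions come from dividing the viewport size, while their dimensions are fixed, so the cross's alignment shifts with resolution.
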(event EventDrawHUD
  (params (SizeX :type Integer) (SizeY :type Integer))
  (HUD|DrawRect self "(R=0.577581,G=0.000000,B=0.396755,A=1.000000)" (/ (Math|Conversions|ToFloat(Integer) SizeX) 2.04) (/ (Math|Conversions|ToFloat(Integer) SizeY) 2.0) 2e+01 2.0)
  (HUD|DrawRect "(R=0.577581,G=0.000000,B=0.396755,A=1.000000)" (/ (Math|Conversions|ToFloat(Integer) SizeX) 2.0) (/ (Math|Conversions|ToFloat(Integer) SizeY) 2.06) 2.0 2e+01))

(fn ConstructionScript)